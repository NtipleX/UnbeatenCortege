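; BP_Tank is a player-controllable tank that drives and aims from input.
; Forward, Right and Brake inputs feed throttle, steering and handbrake on the VehicleMovement component.
; LoockRight yaws the Tower and LoockUp pitches the Cannon, each scaled by a look-speed variable.
; Mouse axes rotate the SpringArm directly, so the camera orbits independently of turret aim, with no clamping in the graph.
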(event EventBeginPlay)

(event Collision|EventActorBeginOverlap
  (params (OtherActor :type Actor%20Object%20Reference)))

(event EventTick
  (params (DeltaSeconds :type Float%20%28single-precision%29)))

(event Input|ActionEvents|InputActionBrake
  (params (Key :type Key%20Structure))
  (bind _vehiclemovement (Variables|Default|GetVehicleMovement))
  (:Pressed
    (Class|WheeledVehicleMovementComponent|SetHandbrakeInput _vehiclemovement true))
  (:Released
    (Class|WheeledVehicleMovementComponent|SetHandbrakeInput _vehiclemovement false)))

(event Input|AxisEvents|InputAxisForward
  (params (AxisValue :type Float%20%28single-precision%29))
  (Class|WheeledVehicleMovementComponent|SetThrottleInput (Variables|Default|GetVehicleMovement) AxisValue))

(event Input|AxisEvents|InputAxisRight
  (params (AxisValue :type Float%20%28single-precision%29))
  (Class|WheeledVehicleMovementComponent|SetSteeringInput (Variables|Default|GetVehicleMovement) AxisValue))

(event Input|AxisEvents|InputAxisLoockRight
  (params (AxisValue :type Float%20%28single-precision%29))
  ;[1 1 1] Tower
  (Transformation|AddLocalRotation (Variables|Default|GetTower) (Math|Rotator|MakeRotator 0.0 0.0 (* AxisValue (Variables|Default|GetLookSpeedX))) false false))

(event Input|AxisEvents|InputAxisLoockUp
  (params (AxisValue :type Float%20%28single-precision%29))
  ;[1 1 1] Tower
  (Transformation|AddLocalRotation (Variables|Default|GetCannon) (Math|Rotator|MakeRotator 0.0 (* AxisValue (Variables|Default|GetLookSpeedY)) 0.0) false false))

(event Input|MouseEvents|MouseX
  (params (AxisValue :type Float%20%28single-precision%29))
  ;[1 1 1] Cam
  (Transformation|AddRelativeRotation (Variables|Default|GetSpringArm) (Math|Rotator|MakeRotator 0.0 0.0 AxisValue) false false))

(event Input|MouseEvents|MouseY
  (params (AxisValue :type Float%20%28single-precision%29))
  ;[1 1 1] Cam
  (Transformation|AddRelativeRotation (Variables|Default|GetSpringArm) (Math|Rotator|MakeRotator 0.0 AxisValue 0.0) false false))

(fn ConstructionScript)