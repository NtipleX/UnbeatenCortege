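; Heavy enemy soldier character with attached helmet and armor that detects the hero and feeds its AI blackboard.
; Sight perception is confirmed by a line trace ignoring BP_EnemySoldier actors, setting VisibleHero or forgetting targets after a short delay when blocked.
; Hits record the player's location in the blackboard and spawn blood at zero health, while death randomly drops a coin.
; HasSeenPlayerBeforeDeath reports whether VisibleHero is set, flagging death when it is not.
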(event Custom|nxPerceptionUpdate
  (params (UpdatedActors :type Array%20of%20Actor%20Object%20References))
  (bind _returnvalue (Pawn|GetController))
  (bind _returnvalue_2 (Utilities|Name|MakeLiteralName "VisibleHero"))
  (bind _self self)
  (bind _aiperception_0 (Variables|Default|GetAIPerception_0))
  (bind _outactors (Class|AIPerceptionComponent|GetPerceivedActors _aiperception_0 "/Script/AIModule.AISense_Sight"))
  (bind _returnvalue_3 (AI|GetAIController _self))
  (if (!= (Utilities|Array|Length _outactors) 0)
    (bind _outactors_2 (Actor|GetAllActorsOfClass "/Game/Game/Characters/AI/BP_EnemySoldier.BP_EnemySoldier_C"))
    (bind _outhit (Collision|LineTraceByChannel (- (Transformation|GetActorLocation) "0, 0,20.000000") (- (Transformation|GetActorLocation (Utilities|Array|Get(acopy) _outactors (Utilities|Array|LastIndex _outactors))) "0, 0,20.000000") "TraceTypeQuery1" false _outactors_2 "None"))
    (bind _asbp_hero (Utilities|Casting|CastToBP_Hero (.HitActor (Collision|BreakHitResult _outhit)))
      (:then
        (if (Utilities|IsValid _returnvalue)
          (AI|Components|Blackboard|SetValueasObject (AI|GetBlackboard _returnvalue) _returnvalue_2 _asbp_hero)))
      (:CastFailed
        (Utilities|FlowControl|Delay 0.2)
        (Class|AIPerceptionComponent|ForgetAll (Variables|Default|GetAIPerception_0))
        (Utilities|IsValid _returnvalue_3
          (:Is%20Valid
            (AI|Components|Blackboard|ClearValue (AI|GetBlackboard _returnvalue_3) _returnvalue_2)))))))

(event Custom|OnEnemyHit_BP
  (bind _returnvalue (Pawn|GetController))
  (if (Utilities|IsValid _returnvalue)
    (AI|Components|Blackboard|SetValueasVector (AI|GetBlackboard _returnvalue) (Utilities|Name|MakeLiteralName "PlayerHitLocation") (Transformation|GetActorLocation (Game|Player|GetPlayerPawn 0)))
    (if (<= (Variables|Default|GetheroHealth) 0.0)
      (Effects|SpawnEmitteratLocation "/Game/Assets/VFX/P_ImpactBlood.P_ImpactBlood" (Transformation|GetActorLocation) (Transformation|GetActorRotation) "0.700000,0.700000,0.700000"))))

(event Custom|SwitchRotation
  (params (IsAlerted :type Boolean))
  (Variables|/Script/Engine.CharacterMovementComponent|SetbOrientRotationToMovement (Variables|Character|GetCharacterMovement) (not IsAlerted)))

(event Custom|SpawnCoin
  (if (== (Math|Random|RandomIntegerinRange 0 5) 0)
    (Game|SpawnActorfromClass "/Game/Game/Blueprints/Misc/CoinDrop.CoinDrop_C" (Math|Transform|MakeTransform (Transformation|GetActorLocation)) "Undefined" 0 0)))

(event EventBeginPlay
  (bind _mesh (Variables|Character|GetMesh))
  (bind _helmet (Variables|Default|GetHelmet))
  (bind _armor (Variables|Default|GetArmor))
  (EventDispatchers|BindEventtoOnPerceptionUpdated (Variables|Default|GetAIPerception_0) (delegate Custom|nxPerceptionUpdate))
  (EventDispatchers|BindEventtoOnEnemyHit (delegate Custom|OnEnemyHit_BP))
  (bind _aswbp_healthbar_1 (Utilities|Casting|CastToWBP_Healthbar1 (UserInterface|GetWidget (Variables|Default|GetheroHealthbar))))
  (Variables|/Game/Game/Blueprints/Widgets/WBP_Healthbar1.WBP_Healthbar1_C|SetOwner _aswbp_healthbar_1 self)
  (EventDispatchers|AssignOnSoldierDead (delegate Custom|SpawnCoin))
  (Transformation|AttachComponentToComponent _helmet _mesh "HelmetSocket" "KeepRelative" "KeepRelative" "KeepRelative" true)
  (Transformation|ResetRelativeTransform _helmet)
  (Transformation|AttachComponentToComponent _armor _mesh "ArmorSocket" "KeepRelative" "KeepRelative" "KeepRelative" true)
  (Transformation|ResetRelativeTransform _armor))

(fn ConstructionScript)

(fn HasSeenPlayerBeforeDeath
  (bind _returnvalue (Pawn|GetController))
  (bind _returnvalue_2 (Utilities|Name|MakeLiteralName "VisibleHero"))
  (bind _returnvalue_3 (AI|GetAIController _returnvalue))
  (bind _returnvalue_4 (AI|GetBlackboard _returnvalue_3))
  (bind _returnvalue_5 (AI|Components|Blackboard|GetValueasObject _returnvalue_4 _returnvalue_2))
  (bind _returnvalue_6 (Utilities|IsValid _returnvalue_5))
  (if _returnvalue_6
    _
    (else
      (Variables|Default|Setm_isDead true)))
  (return _returnvalue_6))