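; BP_EnemySoldier is an AI enemy soldier that reports sighted heroes to its Blackboard.
; On each AI perception update, it line traces on Visibility to the last updated actor, with both ends lowered and debug drawing on.
; A BP_Hero hit is written to the VisibleHero key; any other result makes perception forget all, leaving the key untouched.
; The empty-array check is disconnected.
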(event Custom|nxPerceptionUpdate
  (params (UpdatedActors :type Array%20of%20Actor%20Object%20References))
  (bind _outhit (Collision|LineTraceByChannel (- (Transformation|GetActorLocation) "0, 0,30.000000") (- (Transformation|GetActorLocation (Utilities|Array|Get(acopy) UpdatedActors (Utilities|Array|LastIndex UpdatedActors))) "0, 0,30.000000") "TraceTypeQuery1" false 0 "ForDuration" true "(R=1.000000,G=0.000000,B=0.000000,A=1.000000)" "(R=0.000000,G=1.000000,B=0.000000,A=1.000000)" 3.0))
  (bind _asbp_hero (Utilities|Casting|CastToBP_Hero (.HitActor (Collision|BreakHitResult _outhit)))
    (:then
      (AI|Components|Blackboard|SetValueasObject (AI|GetBlackboard (Pawn|GetController)) (Utilities|Name|MakeLiteralName "VisibleHero") _asbp_hero))
    (:CastFailed
      (Class|AIPerceptionComponent|ForgetAll (Variables|Default|GetAIPerception)))))

(event EventBeginPlay
  (EventDispatchers|BindEventtoOnPerceptionUpdated (Variables|Default|GetAIPerception) (delegate Custom|nxPerceptionUpdate)))

(event Collision|EventActorBeginOverlap
  (params (OtherActor :type Actor%20Object%20Reference)))

(event EventTick
  (params (DeltaSeconds :type Float%20%28single-precision%29)))

(fn ConstructionScript)