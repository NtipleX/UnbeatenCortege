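; Game mode that handles level progression, game over and mission completion.
; On BeginPlay it parses episode and stage from the level name, which LoadNextLevel uses to open the following stage, only printing at stage 5.
; Game over pauses the game and frees the cursor via nxPController.
; Winning disables input, blends to the second CameraActor found, then shows a centered WBP_MissionComplete after a delay.
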(event Custom|TriggerGameOver
  (bind _returnvalue (Game|GetPlayerController 0))
  (Development|PrintString "GameOver" true true "(R=0.130349,G=0.503413,B=1.000000,A=1.000000)" 7.0)
  (Game|SetGamePaused true)
  (Actor|Tick|SetActorTickEnabled _returnvalue)
  (bind _asnx_pcontroller (Utilities|Casting|CastTonxPController _returnvalue))
  (Class|NxPController|MakeMouseCursor _asnx_pcontroller))

(event Custom|LoadNextLevel
  (bind _stage (Variables|Default|GetStage))
  (if (== _stage 5)
    (Development|PrintString "GameMode Levels" true true "(R=1.000000,G=0.220697,B=0.330514,A=1.000000)" 1e+01)
    (else
      (bind _result (Math|Integer|IncrementInt _stage)
        (:%20%20
          (Game|OpenLevel(byName) (Utilities|String|StringToName (Utilities|String|Append "lvl" (Utilities|String|ToString(Integer) (Variables|Default|GetEpisode)) "-" (Utilities|String|ToString(Integer) _result)))))))))

(event EventBeginPlay
  (bind _returnvalue (Game|GetCurrentLevelName true))
  (Variables|Default|SetStage (Math|Conversions|ToInteger(Byte) (.RightS (Utilities|String|Split (Utilities|String|GetSubstring _returnvalue 3 3) "-"))))
  (Variables|Default|SetEpisode (Math|Conversions|ToInteger(Byte) (.LeftS (Utilities|String|Split (Utilities|String|GetSubstring _returnvalue 3 3) "-")))))

(event EventTick
  (params (DeltaSeconds :type Float%20%28single-precision%29)))

(event EventGameOverEvent
  (bind _returnvalue (Game|GetPlayerController 0))
  (Development|PrintString "GameOver" true true "(R=0.130349,G=0.503413,B=1.000000,A=1.000000)" 7.0)
  (Game|SetGamePaused true)
  (Actor|Tick|SetActorTickEnabled _returnvalue)
  (bind _asnx_pcontroller (Utilities|Casting|CastTonxPController _returnvalue))
  (Class|NxPController|MakeMouseCursor _asnx_pcontroller))

(event EventGameWinEvent
  (bind _returnvalue (Game|GetPlayerController 0))
  (bind _returnvalue_2 (Game|GetPlayerController 0))
  (Actor|Tick|SetActorTickEnabled _returnvalue)
  (Input|DisableInput (Game|GetPlayerCharacter 0) _returnvalue)
  (bind _outactors (Actor|GetAllActorsOfClass "/Script/Engine.CameraActor"))
  (Game|Player|SetViewTargetwithBlend _returnvalue_2 (Utilities|Array|Get(acopy) _outactors 1) 1.2 "VTBlend_Cubic" 0.0 false)
  (bind _asnx_pcontroller (Utilities|Casting|CastTonxPController _returnvalue_2))
  (Class|NxPController|MakeMouseCursor _asnx_pcontroller)
  (Utilities|FlowControl|Delay 2.5)
  (bind _returnvalue_3 (UserInterface|CreateWidget "/Game/Game/Blueprints/Widgets/WBP_MissionComplete.WBP_MissionComplete_C"))
  (Widget|SetVisibility _returnvalue_3 "Hidden")
  (UserInterface|Viewport|AddtoViewport _returnvalue_3 0)
  (Utilities|FlowControl|Delay 0.1)
  (Class|UserWidget|SetPositioninViewport _returnvalue_3 (- (/ (Viewport|GetViewportSize) 2.0) (/ (Class|Widget|GetDesiredSize _returnvalue_3) 2.0)) true)
  (Widget|SetVisibility _returnvalue_3 "Visible"))

(fn ConstructionScript)