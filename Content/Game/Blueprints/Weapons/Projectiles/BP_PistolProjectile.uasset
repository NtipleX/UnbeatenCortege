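; BP_PistolProjectile is a pistol projectile actor Blueprint, built from three static meshes and a rect light.
; Its only active logic is the HideShit event, which hides those four components in game and then destroys them to strip the projectile's visuals.
; No movement, collision or damage logic appears in this graph, and nothing here calls that event.
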(event EventBeginPlay)

(event Collision|EventActorBeginOverlap
  (params (OtherActor :type Actor%20Object%20Reference)))

(event EventTick
  (params (DeltaSeconds :type Float%20%28single-precision%29)))

(event EventHideShit
  (bind _staticmesh1 (Variables|Default|GetStaticMesh1))
  (bind _staticmesh2 (Variables|Default|GetStaticMesh2))
  (bind _staticmesh (Variables|Default|GetStaticMesh))
  (bind _rectlight (Variables|Default|GetRectLight))
  (Development|SetHiddeninGame _staticmesh true false)
  (Development|SetHiddeninGame _staticmesh1 true false)
  (Development|SetHiddeninGame _staticmesh2 true false)
  (Development|SetHiddeninGame _rectlight true false)
  (Components|DestroyComponent _staticmesh)
  (Components|DestroyComponent _staticmesh1)
  (Components|DestroyComponent _staticmesh2)
  (Components|DestroyComponent _rectlight))

(fn ConstructionScript)