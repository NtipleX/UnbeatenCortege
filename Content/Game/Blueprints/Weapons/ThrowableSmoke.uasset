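; Throwable smoke grenade that launches itself with a forward and upward impulse on spawn, then deploys smoke after a short fuse.
; A timer plays a pop sound and activates two particle systems, whose world scale grows along the SmokeScale timeline.
; After a hold, a second timer reverses the timeline once to shrink the smoke, guarded by a boolean; the actor is never destroyed here.
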(event Custom|MakeSmoke
  (Audio|PlaySound2D "/Game/Assets/SFX/GunShots/Explosion_Tiny_6.Explosion_Tiny_6" 1.0 1.0 0.0 0 0)
  (Components|Activation|Activate (Variables|Default|GetParticleSystem) true)
  (Components|Activation|Activate (Variables|Default|GetParticleSystem1) true)
  (bind _smokescale (Timeline|SmokeScale PlayFromStart)
    (:Update
      (Transformation|SetWorldScale3D (Variables|Default|GetParticleSystem) (Math|Vector|MakeVector _smokescale _smokescale _smokescale))
      (Transformation|SetWorldScale3D (Variables|Default|GetParticleSystem1) (Math|Vector|MakeVector _smokescale _smokescale _smokescale)))
    (:Finished
      (Utilities|Time|SetTimerbyEvent (delegate Custom|CustomEvent_0) 28.0))))

(event Custom|CustomEvent_0
  (if (not (Variables|Default|GetNewVar_0))
    (Variables|Default|SetNewVar_0 true)
    (bind _smokescale (Timeline|SmokeScale ReverseFromEnd)
      (:Update
        (Transformation|SetWorldScale3D (Variables|Default|GetParticleSystem) (Math|Vector|MakeVector _smokescale _smokescale _smokescale))
        (Transformation|SetWorldScale3D (Variables|Default|GetParticleSystem1) (Math|Vector|MakeVector _smokescale _smokescale _smokescale)))
      (:Finished
        (Utilities|Time|SetTimerbyEvent (delegate Custom|CustomEvent_0) 28.0)))))

(event EventBeginPlay
  (bind _returnvalue (Transformation|GetActorRotation))
  (bind _returnvalue_2 (Math|Vector|GetForwardVector _returnvalue))
  (bind _returnvalue_3 (* _returnvalue_2 "0.450000,0.450000,0.500000"))
  (bind (_x _y) (Math|Vector|BreakVector _returnvalue_3))
  (Physics|AddImpulse (Variables|Default|Getr) (Math|Vector|MakeVector _x _y 0.35) "None" false)
  (Utilities|Time|SetTimerbyEvent (delegate Custom|MakeSmoke) 1.0))

(event Collision|EventActorBeginOverlap
  (params (OtherActor :type Actor%20Object%20Reference)))

(event EventTick
  (params (DeltaSeconds :type Float%20%28single-precision%29)))

(fn ConstructionScript)