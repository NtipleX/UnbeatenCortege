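; LeftFootDecal is a left footprint decal actor that fades partially over time.
; On BeginPlay it gives its decal component a dynamic material instance and starts a timer.
; Two chained one-shot timers then lower the material's Opacity parameter in steps, leaving it semi-transparent without destroying the actor.
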(event Custom|Dissapear1
  (bind _asmaterial_instance_dynamic (Utilities|Casting|CastToMaterialInstanceDynamic (Class|DecalComponent|GetDecalMaterial (Variables|Default|GetDecal))))
  (Rendering|Material|SetScalarParameterValue _asmaterial_instance_dynamic "Opacity" 0.75 :!class /Script/Engine.MaterialInstanceDynamic)
  (Utilities|Time|SetTimerbyEvent (delegate Custom|Dissapear2) 1e+01))

(event Custom|Dissapear2
  (bind _asmaterial_instance_dynamic (Utilities|Casting|CastToMaterialInstanceDynamic (Class|DecalComponent|GetDecalMaterial (Variables|Default|GetDecal))))
  (Rendering|Material|SetScalarParameterValue _asmaterial_instance_dynamic "Opacity" 0.5 :!class /Script/Engine.MaterialInstanceDynamic))

(event EventBeginPlay
  (bind _decal (Variables|Default|GetDecal))
  (Utilities|Time|SetTimerbyEvent (delegate Custom|Dissapear1) 5.0)
  (bind _returnvalue (Rendering|Material|CreateDynamicMaterialInstance (Class|DecalComponent|GetDecalMaterial _decal) "None" "None" :!class /Script/Engine.KismetMaterialLibrary))
  (Rendering|Components|Decal|SetDecalMaterial _decal _returnvalue))

(fn ConstructionScript)