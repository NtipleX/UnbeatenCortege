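; MoneyEffect is a short-lived cosmetic actor, apparently a money popup, that drifts upward and fades out.
; BeginPlay creates a dynamic material instance on its static mesh and destroys the actor after a fixed delay.
; Tick applies a fixed per-frame local offset, so drift speed depends on frame rate.
; It also drives the material's Opacity2 parameter from a clamped, delta-time-based countdown variable.
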(event EventBeginPlay
  (Rendering|Material|CreateDynamicMaterialInstance (Variables|Default|GetStaticMesh) 0 0 "None" :!class /Script/Engine.PrimitiveComponent)
  (Utilities|FlowControl|Delay 3.5)
  (Actor|DestroyActor))

(event Collision|EventActorBeginOverlap
  (params (OtherActor :type Actor%20Object%20Reference)))

(event EventTick
  (params (DeltaSeconds :type Float%20%28single-precision%29))
  (Transformation|AddActorLocalOffset "-0.300000,0.000000,2.000000" false true)
  (bind _asmaterial_instance_dynamic (Utilities|Casting|CastToMaterialInstanceDynamic (Rendering|Material|GetMaterial (Variables|Default|GetStaticMesh) 0)))
  (Rendering|Material|SetScalarParameterValue _asmaterial_instance_dynamic "Opacity2" (/ (Variables|Default|GetNewVar_0) 3.0) :!class /Script/Engine.MaterialInstanceDynamic)
  (Variables|Default|SetNewVar_0 (Math|Float|Clamp(Float) (- (Variables|Default|GetNewVar_0) (* 4 DeltaSeconds)) 0.0 3.0)))

(fn ConstructionScript)